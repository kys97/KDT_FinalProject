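; BP_StormText is a visual-effect actor that scales up a particle component, MParticle, as it plays.
; BeginPlay applies the starting Scale to MParticle, then activates it after a short delay.
; While the particle is active, Tick grows its uniform scale using delta time and FadeSpeed until Scale reaches about one.
; The overlap event, labeled Damage, and the construction script are empty.
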(event EventBeginPlay
  ;[1 1 1] Active
  (Transformation|SetRelativeScale3D (Variables|Default|GetmParticle) (* (Variables|Default|GetScale) (Class|KismetMathLibrary|VectorOne)))
  (Utilities|FlowControl|Delay 1.0)
  (Components|Activation|Activate (Variables|Default|GetmParticle) false))

(event Collision|EventActorBeginOverlap
  (params (OtherActor :type Actor%20Object%20Reference))
  ;[1 1 1] Damage
)

(event EventTick
  (params (DeltaSeconds :type Float%20%28single-precision%29))
  ;[1 1 1] Add Size
  (if (Components|Activation|IsActive (Variables|Default|GetmParticle))
    (Utilities|FlowControl|ForLoopwithBreak 0 0 :!label _label
      (:LoopBody
        (if (< (Variables|Default|GetScale) 1.0)
          (bind _output_get (Variables|Default|SetScale (+ (* (Utilities|Time|GetWorldDeltaSeconds) (Variables|Default|GetFadeSpeed)) (Variables|Default|GetScale))))
          (Transformation|SetRelativeScale3D (Variables|Default|GetmParticle) (* _output_get (Class|KismetMathLibrary|VectorOne)))
          (else
            (goto _label Break)))))))

(fn ConstructionScript)