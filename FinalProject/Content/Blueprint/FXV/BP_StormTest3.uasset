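; BP_StormTest3 is a test storm effect actor built around a particle system that grows in after spawning.
; On BeginPlay it applies the starting scale to the particle component, then activates it after a short delay.
; While the system is active, Tick raises the uniform scale at FadeSpeed until it reaches about full size.
; Actor overlaps only print the other actor on screen.
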(event EventBeginPlay
  ;[1 1 1] Active
  (Transformation|SetRelativeScale3D (Variables|Default|GetParticleSystem) (* (Variables|Default|GetScale) (Class|KismetMathLibrary|VectorOne)))
  (Utilities|FlowControl|Delay 1.0)
  (Components|Activation|Activate (Variables|Default|GetParticleSystem) false))

(event Collision|EventActorBeginOverlap
  (params (OtherActor :type Actor%20Object%20Reference))
  (Development|PrintText (Utilities|Text|ToText(Object) OtherActor) true false))

(event EventTick
  (params (DeltaSeconds :type Float%20%28single-precision%29))
  ;[1 1 1] Add Size
  (if (Components|Activation|IsActive (Variables|Default|GetParticleSystem))
    (if (< (Variables|Default|GetScale) 1.0)
      (bind _output_get (Variables|Default|SetScale (+ (* DeltaSeconds (Variables|Default|GetFadeSpeed)) (Variables|Default|GetScale))))
      (Transformation|SetRelativeScale3D (Variables|Default|GetParticleSystem) (* _output_get (Class|KismetMathLibrary|VectorOne))))))

(fn ConstructionScript)