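; BP_StormTest2 is a test actor, apparently for a storm effect, with an incomplete grow-in.
; Tick raises Scale by DeltaSeconds times FadeSpeed while it is below 1, but the graph never applies the value, as both vector multiply nodes are unused.
; Overlapping actors are printed as debug text, BeginPlay and the construction script are empty, and a Delay node is unconnected.
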(event EventBeginPlay
  ;[1 1 1] Active
)

(event Collision|EventActorBeginOverlap
  (params (OtherActor :type Actor%20Object%20Reference))
  (Development|PrintText (Utilities|Text|ToText(Object) OtherActor) true false))

(event EventTick
  (params (DeltaSeconds :type Float%20%28single-precision%29))
  ;[1 1 1] Add Size
  (if true
    (if (< (Variables|Default|GetScale) 1.0)
      (bind _output_get (Variables|Default|SetScale (+ (* DeltaSeconds (Variables|Default|GetFadeSpeed)) (Variables|Default|GetScale)))))))

(fn ConstructionScript)